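; BP_VRHands is a VR hand-tracking Blueprint that converts motion controller data into per-joint transforms.
; GetJointTransforms checks that the data is valid, comes from a tracked hand rather than a controller, and has 26 key positions and rotations.
; It then pairs them into transforms at a small uniform scale.
; Tick currently only prints the left hand's joint count, apparently as a debug readout.
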(event `self.ReceiveTick`
  (params (DeltaSeconds :type "Float (single-precision)"))
  (bind _transforms (`self.Get Joint Transforms` "Left"))
  (`KismetSystemLibrary.PrintString` (`KismetStringLibrary.Conv_IntToString` (`KismetArrayLibrary.Array_Length` _transforms))))

(fn `Get Joint Transforms`
  (params (Hand :type "EControllerHand Enum" :default "Left"))
  (returns (Transforms :type "Array of Transform Structure"))
  (locals (`Joint Transforms` :type "Array of Transform Structure"))
  ;[1 1 1] Get the actual hand-tracking data
  (bind _motioncontrollerdata (`HeadMountedDisplayFunctionLibrary.GetMotionControllerData` null Hand))
  (bind (_bvalid _devicename _applicationinstanceid _devicevisualtype _handindex _trackingstatus _gripposition _griprotation _aimposition _aimrotation _palmposition _palmrotation _handkeypositions _handkeyrotations) (break `XRMotionControllerData` _motioncontrollerdata))
  ;[1 1 1] Perform data validation
  (if _bvalid
    (switch `EXRVisualType` _devicevisualtype
      (:`Controller`
        _)
      (:`Hand`
        (if (and (== (`KismetArrayLibrary.Array_Length` _handkeypositions) 26) (== (`KismetArrayLibrary.Array_Length` _handkeyrotations) 26))
          ;[1 1 1] create joint transform array and add translations and rotations
          (for (_ _array_index) _handkeypositions
            (`KismetArrayLibrary.Array_Add` (`local.Joint Transforms`) (`KismetMathLibrary.MakeTransform` (`|GetArrayItem` _handkeypositions _array_index) (`KismetMathLibrary.Quat_Rotator` (`|GetArrayItem` _handkeyrotations _array_index)) (0.01 0.01 0.01))))
          (return (`local.Joint Transforms`))
          (else
            _))))
    (return)))

(fn `UserConstructionScript`)